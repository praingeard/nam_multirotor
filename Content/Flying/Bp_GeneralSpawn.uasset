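; Spawner actor in the Flying game folder that places blockers as child actors at five spawn points.
; When an overlap ends, it stores the points' relative transforms in an array and adds a child actor component at each.
; It destroys all child actors two seconds later, or immediately when an overlap begins.
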(event Collision|EventActorEndOverlap
  (params (OtherActor :type Actor%20Object%20Reference))
  (CallFunction|SpawnObstacle)
  (CallFunction|SpawnBlockers)
  (Utilities|FlowControl|Delay 2.0)
  (Actor|DestroyActor (Actor|GetAllChildActors true)))

(event Collision|EventActorBeginOverlap
  (params (OtherActor :type Actor%20Object%20Reference))
  (Actor|DestroyActor (Actor|GetAllChildActors true)))

(fn ConstructionScript)

(fn SpawnObstacle
  (Variables|Default|SetSpawn%20Points (Utilities|Array|MakeArray (Transformation|GetRelativeTransform (Variables|Default|GetSpawnPoint1)) (Transformation|GetRelativeTransform (Variables|Default|GetSpawnPoint2)) (Transformation|GetRelativeTransform (Variables|Default|GetSpawnPoint3)) (Transformation|GetRelativeTransform (Variables|Default|GetSpawnPoint4)) (Transformation|GetRelativeTransform (Variables|Default|GetSpawnPoint5)))))

(fn SpawnBlockers
  (for _array_element (Variables|Default|GetSpawn%20Points)
    (AddComponent|AddChildActorComponent false _array_element)))